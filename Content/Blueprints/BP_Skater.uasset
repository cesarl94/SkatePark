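; BP_Skater is the skater Blueprint that plays the skateboarding animations for impulse, jump, stop and backflip.
; Each action has its own event that plays a montage on the Mesh from a preset start position, with the stop montage also sped up.
; The graph holds no input, movement or state logic and nothing in it calls these events, and the construction script is empty.
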(event EventStartStopAnimation
  (Animation|Montage|PlayMontage (Variables|Character|GetMesh) "/Game/Character/Animations/AM_Stop.AM_Stop" 1.5 0.8))

(event EventStartBackflipAnimation
  (Animation|Montage|PlayMontage (Variables|Character|GetMesh) "/Game/Character/Animations/AM_Backflip.AM_Backflip" 1.0 1.0))

(event EventStartImpulseAnimation
  (Animation|Montage|PlayMontage (Variables|Character|GetMesh) "/Game/Character/Animations/AM_ImpulseOnSkate.AM_ImpulseOnSkate" 1.0 1.15))

(event EventStartJumpAnimation
  (Animation|Montage|PlayMontage (Variables|Character|GetMesh) "/Game/Character/Animations/AM_Jumping.AM_Jumping" 1.0 0.2))

(fn ConstructionScript)
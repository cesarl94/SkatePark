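; Player controller for the skate park that turns Enhanced Input into actions on the possessed BP_Skater pawn.
; BeginPlay registers the IMP_Skaters mapping context on the local player's input subsystem.
; Look input drives the pawn's controller yaw and pitch, while the impulse and jump actions call the skater's Impulse and StartJump after casting the controlled pawn.
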(event Input|EnhancedActionEvents|EnhancedInputActionIA_Impulse
  (params (ActionValue :type Boolean) (ElapsedSeconds :type Float%20%28double-precision%29) (TriggeredSeconds :type Float%20%28double-precision%29) (InputAction :type Input%20Action%20Object%20Reference :default "/Game/Input/Actions/IA_Impulse.IA_Impulse"))
  (if ActionValue
    (bind _asbp_skater (Utilities|Casting|CastToBP_Skater (Pawn|GetControlledPawn)))
    (Default|Impulse _asbp_skater)))

(event Input|EnhancedActionEvents|EnhancedInputActionIA_Look
  (params (ActionValue :type Vector%202D%20Structure) (ElapsedSeconds :type Float%20%28double-precision%29) (TriggeredSeconds :type Float%20%28double-precision%29) (InputAction :type Input%20Action%20Object%20Reference :default "/Game/Input/Actions/IA_Look.IA_Look"))
  (bind _asbp_skater (Utilities|Casting|CastToBP_Skater (Pawn|GetControlledPawn)))
  (Pawn|Input|AddControllerYawInput _asbp_skater (.x ActionValue))
  (Pawn|Input|AddControllerPitchInput _asbp_skater (.y ActionValue)))

(event Input|EnhancedActionEvents|EnhancedInputActionIA_Jump
  (params (ActionValue :type Boolean) (ElapsedSeconds :type Float%20%28double-precision%29) (TriggeredSeconds :type Float%20%28double-precision%29) (InputAction :type Input%20Action%20Object%20Reference :default "/Game/Input/Actions/IA_Jump.IA_Jump"))
  (if ActionValue
    (bind _asbp_skater (Utilities|Casting|CastToBP_Skater (Pawn|GetControlledPawn)))
    (Default|StartJump _asbp_skater false)))

(event EventBeginPlay
  (bind _returnvalue (PlayerController|LocalPlayerSubsystems|GetEnhancedInputLocalPlayerSubsystem))
  (Utilities|IsValid _returnvalue
    (:Is%20Valid
      (Input|AddMappingContext _returnvalue "/Game/Input/IMP_Skaters.IMP_Skaters" 0 "(bIgnoreAllPressedKeysUntilRelease=True,bForceImmediately=False,bNotifyUserSettings=False)"))))

(event EventTick
  (params (DeltaSeconds :type Float%20%28single-precision%29)))

(fn ConstructionScript)
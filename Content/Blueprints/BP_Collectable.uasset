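; BP_Collectable is a collectable pickup actor with a spinning star, a circle and a particle effect.
; Each tick it yaws the star and bobs the visual scene component with a sine of server world time, keeping the motion in step across clients.
; StartCollectAnimation hides the star and circle and plays the particles, and the actor destroys itself when the system finishes.
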(event Custom|#OnParticlesFinished
  (params (PSystem :type Niagara%20Component%20Object%20Reference))
  (Actor|DestroyActor))

(event EventTick
  (params (DeltaSeconds :type Float%20%28single-precision%29))
  (Transformation|AddRelativeRotation (Variables|Default|GetStar) (Math|Rotator|MakeRotator 0.0 0.0 (* DeltaSeconds 1.2e+02)) false false)
  (Transformation|SetRelativeLocation (Variables|Default|GetVisualSceneComponent) (Math|Vector|MakeVector 0.0 0.0 (* (Math|Trig|Sin(Radians) (* (GameState|GetServerWorldTimeSeconds (Game|GetGameState)) 2.0)) 1e+01)) false false))

(event EventStartCollectAnimation
  (bind _particles (Variables|Default|GetParticles))
  (EventDispatchers|BindEventtoOnSystemFinished _particles (EventDispatchers|CreateEvent :!event Custom|#OnParticlesFinished))
  (Components|Activation|Activate _particles false)
  (Rendering|SetVisibility (Variables|Default|GetCircle) false false)
  (Rendering|SetVisibility (Variables|Default|GetStar) false false))

(fn ConstructionScript)
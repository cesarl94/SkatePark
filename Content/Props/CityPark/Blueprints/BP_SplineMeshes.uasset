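; Spline-driven prop Blueprint in the CityPark set that repeats a mesh along a spline, bent to follow its curve.
; The construction script adds a spline mesh component per segment and applies two material slots.
; SplineMeshVar selects segmentation: one piece per pair of spline points using their tangents, or pieces at fixed Spacing intervals.
; Spacing mode scales tangents from spline direction by spacing plus an adjustable offset.
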(fn ConstructionScript
  (|Wire))